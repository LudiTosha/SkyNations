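; BP_HoverBoat is a hover boat vehicle Blueprint that sets up its hover behavior when play begins.
; On BeginPlay it initializes six BPHoverComponent instances, passing the same Cube component to each as their shared body.
; The hover logic lives in those components, as this Blueprint has an empty construction script and no other graph logic.
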(event EventBeginPlay
  (bind _cube (Variables|Default|GetCube))
  (bind _cube_2 (Variables|Default|GetCube))
  (bind _cube_3 (Variables|Default|GetCube))
  (Default|InitComponent (Variables|Default|GetBP_HoverComponent) _cube_2)
  (Default|InitComponent (Variables|Default|GetBP_HoverComponent1) _cube_2)
  (Default|InitComponent (Variables|Default|GetBP_HoverComponent2) _cube_3)
  (Default|InitComponent (Variables|Default|GetBP_HoverComponent3) _cube_3)
  (Default|InitComponent (Variables|Default|GetBP_HoverComponent4) _cube)
  (Default|InitComponent (Variables|Default|GetBP_HoverComponent5) _cube))

(fn ConstructionScript)