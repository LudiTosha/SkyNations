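; BP_Ship is a vehicle Blueprint for a ship that carries six hover components.
; On BeginPlay it initializes each hover component, passing the same Ship reference to all six.
; The graph holds only this wiring, so any hover behavior lives in the components, and the construction script is empty.
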(event EventBeginPlay
  (bind _ship (Variables|Default|GetShip))
  (bind _ship_2 (Variables|Default|GetShip))
  (bind _ship_3 (Variables|Default|GetShip))
  (Default|InitComponent (Variables|Default|GetBP_HoverComponent2) _ship_2)
  (Default|InitComponent (Variables|Default|GetBP_HoverComponent1) _ship_2)
  (Default|InitComponent (Variables|Default|GetBP_HoverComponent) _ship_3)
  (Default|InitComponent (Variables|Default|GetBP_HoverComponent5) _ship_3)
  (Default|InitComponent (Variables|Default|GetBP_HoverComponent4) _ship)
  (Default|InitComponent (Variables|Default|GetBP_HoverComponent3) _ship))

(fn ConstructionScript)